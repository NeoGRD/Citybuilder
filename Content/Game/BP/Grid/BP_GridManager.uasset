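; BP_GridManager is an actor that maps between world positions and integer cells on a flat XY grid anchored at its own location.
; WorldToGrid floors the offset from the actor divided by CellSize, while GridToWorld returns the cell's center at the actor's Z, ignoring actor rotation and scale.
; Tick prints the world position of a hard-coded test cell every frame as debug output.
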(event `self.ReceiveTick`
  (params (DeltaSeconds :type "Float (single-precision)"))
  (bind _position (`self.GridToWorld` (make `IntPoint` 2 1)))
  (`KismetSystemLibrary.PrintString` (`KismetStringLibrary.Conv_VectorToString` _position)))

(fn `GridToWorld`
  (params (Cell :type "IntPoint Structure"))
  (returns (Position :type "Vector Structure"))
  (bind (_x _y) (break `IntPoint` Cell))
  (bind _cellsize (`self.CellSize`))
  (bind _returnvalue (/ _cellsize 2.0))
  (return (`KismetMathLibrary.MakeVector` (+ (* _x (`self.CellSize`)) (.x (`self.K2_GetActorLocation`)) _returnvalue) (+ (* _y _cellsize) (.y (`self.K2_GetActorLocation`)) _returnvalue) (.z (`self.K2_GetActorLocation`)))))

(fn `UserConstructionScript`)

(fn `WorldToGrid`
  (params (Position :type "Vector Structure"))
  (returns (Cell :type "IntPoint Structure"))
  (return (make `IntPoint` (`KismetMathLibrary.FFloor` (/ (- (.x Position) (.x (`self.K2_GetActorLocation`))) (`self.CellSize`))) (`KismetMathLibrary.FFloor` (/ (- (.y Position) (.y (`self.K2_GetActorLocation`))) (`self.CellSize`))))))